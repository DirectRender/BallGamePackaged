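; BP_Star is a collectible star that reports to the game mode when a Player-tagged actor overlaps its sphere.
; A timeline started on BeginPlay animates the Star component's relative location.
; On pickup it sends an add-star message to the game mode, hides PStar and plays a sound.
; A second timeline then raises and yaws the whole actor until it is destroyed after a short delay.
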(event OnComponentBeginOverlap(Sphere)
  (params (OverlappedComponent :type Primitive%20Component%20Object%20Reference) (OtherActor :type Actor%20Object%20Reference) (OtherComp :type Primitive%20Component%20Object%20Reference) (OtherBodyIndex :type Integer) (bFromSweep :type Boolean) (SweepResult :type Hit%20Result%20Structure%20%28by%20ref%29))
  (CallFunction|HittedStar OtherActor))

(event Custom|StarPickuped
  (bind _returnvalue (Transformation|GetActorLocation))
  (bind _returnvalue_2 (Transformation|GetActorRotation))
  (Rendering|SetVisibility (Variables|Default|GetP_Star) false false)
  (Audio|PlaySoundatLocation "/Game/Audio/SFX_Star.SFX_Star" (Transformation|GetWorldLocation (Variables|Default|GetStar)) "0, 0, 0" 1.0 1.0 0.0 0 0 0 0)
  (bind (_direction _locationalpha _rotationalpha) (Timeline|StarPikcupMovement Play)
    (:Update
      (Transformation|SetActorRelativeLocation (Math|Vector|MakeVector (.x _returnvalue) (.y _returnvalue) (+ (.z _returnvalue) (.Z (Math|Vector|BreakVector _locationalpha)))))
      (Transformation|SetActorRelativeRotation (Math|Rotator|MakeRotator (.roll _returnvalue_2) (.pitch _returnvalue_2) _rotationalpha)))))

(event Custom|HittedStar
  (params (Target :type Actor%20Object%20Reference))
  (if (Actor|ActorHasTag Target "Player")
    (bind _gamemode (Class|INTGameMode|GetGameModeRef(Message) (Game|GetGameMode)))
    (Class|INTGameMode|AddStar(Message) _gamemode)
    (CallFunction|StarPickuped)
    (Utilities|FlowControl|Delay 0.5)
    (Actor|DestroyActor)))

(event EventBeginPlay
  (bind _locationalpha (Timeline|StartMovement Play)
    (:Update
      (Transformation|SetRelativeLocation (Variables|Default|GetStar) _locationalpha false false))))

(fn ConstructionScript)

(fn OnRepStars)