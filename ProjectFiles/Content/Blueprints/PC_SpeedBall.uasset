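; Player controller for SpeedBall that creates the main widget on BeginPlay and rolls the player's ball from movement input.
; Each movement axis gets the ball from player pawn 0 through a GetBallRef message and applies mass-independent torque to it.
; The same torque is applied both in a custom event and inline, so each input pushes twice.
; The Restart action reloads the SpeedBall map.
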(event Custom|MoveForwardEvent
  (params (A :type Float%20%28single-precision%29))
  (bind _ball (Class|INTBPBall|GetBallRef(Message) (Game|Player|GetPlayerPawn 0)))
  (bind _ball_2 (Variables|/Game/Blueprints/BP_Ball.BP_Ball_C|GetBall _ball)
    (:then
      (Class|PrimitiveComponent|AddTorqueinRadians _ball_2 (Math|Vector|MakeVector 0.0 (* A 5e+01) 0.0) "None" true))
    (:else)))

(event Custom|MoveRightEvent
  (params (A :type Float%20%28single-precision%29))
  (bind _ball (Class|INTBPBall|GetBallRef(Message) (Game|Player|GetPlayerPawn 0)))
  (bind _ball_2 (Variables|/Game/Blueprints/BP_Ball.BP_Ball_C|GetBall _ball)
    (:then
      (Class|PrimitiveComponent|AddTorqueinRadians _ball_2 (Math|Vector|MakeVector (* A -5e+01) 0.0 0.0) "None" true))
    (:else)))

(event EventBeginPlay
  (bind _returnvalue (UserInterface|CreateWidget "/Game/UI/WB_Maint.WB_Maint_C"))
  (UserInterface|Viewport|AddtoViewport _returnvalue 0))

(event Input|ActionEvents|InputActionRestart
  (params (Key :type Key%20Structure :default "None"))
  (:Pressed
    (Game|OpenLevel(byName) "MAP_SpeedBall")))

(event Input|AxisEvents|InputAxisMoveForward
  (params (AxisValue :type Float%20%28single-precision%29))
  (CallFunction|MoveForwardEvent AxisValue)
  (bind _ball (Class|INTBPBall|GetBallRef(Message) (Game|Player|GetPlayerPawn 0)))
  (bind _ball_2 (Variables|/Game/Blueprints/BP_Ball.BP_Ball_C|GetBall _ball)
    (:then
      (Class|PrimitiveComponent|AddTorqueinRadians _ball_2 (Math|Vector|MakeVector 0.0 (* AxisValue 5e+01) 0.0) "None" true))
    (:else)))

(event Input|AxisEvents|InputAxisMoveRight
  (params (AxisValue :type Float%20%28single-precision%29))
  (CallFunction|MoveRightEvent AxisValue)
  (bind _ball (Class|INTBPBall|GetBallRef(Message) (Game|Player|GetPlayerPawn 0)))
  (bind _ball_2 (Variables|/Game/Blueprints/BP_Ball.BP_Ball_C|GetBall _ball)
    (:then
      (Class|PrimitiveComponent|AddTorqueinRadians _ball_2 (Math|Vector|MakeVector (* AxisValue -5e+01) 0.0 0.0) "None" true))
    (:else)))

(fn ConstructionScript)